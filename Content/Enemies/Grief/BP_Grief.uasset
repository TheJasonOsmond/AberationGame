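; BP_Grief is the Blueprint for the Grief enemy.
; On BeginPlay it casts its controller to AIC_Enemy_Base and caches it, stopping if the cast fails.
; It then binds handlers to the damage system component's OnDeath and OnDamageResponse events.
; The construction script only calls the parent's version.
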(event `self.ReceiveBeginPlay`
  (bind _bpc_damagesystem (`self.BPC_DamageSystem`))
  (bind _asaic_enemy_base (cast `/Game/Enemies/AI/AIC_Enemy_Base` (`AIBlueprintHelperLibrary.GetAIController` self)))
  (set `self.AICEnemyBase` _asaic_enemy_base)
  (add `/Game/DamageSystem/BPC_DamageSystem.OnDeath` _bpc_damagesystem (`|CreateDelegate` :!event `Die`))
  (add `/Game/DamageSystem/BPC_DamageSystem.OnDamageResponse` _bpc_damagesystem (`|CreateDelegate` :!event `HitResponse`)))

(fn `UserConstructionScript`
  (`parent.UserConstructionScript`))