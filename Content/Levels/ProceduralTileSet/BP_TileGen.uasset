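; BP_TileGen is a procedural tile generator that spawns a line of tile actors when play begins.
; CreateTiles reads the tile class from the fixed "Test" row of the Tiles data table, then loops up to TileCountY.
; Each tile takes the level transform, with Y set to the loop count times the sum of level Y and TileStandardOffset.
; Random row selection exists but is unused, and a debug string prints each iteration.
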(event `self.ReceiveBeginPlay`
  (`self.CreateTiles`))

(fn `CreateTiles`
  (locals (Zero :type Integer :default 0) (Index :type Integer))
  (bind _returnvalue (`self.GetLevelTransform`))
  (bind _tiles (`self.Tiles`))
  (bind _outrownames (`DataTableFunctionLibrary.GetDataTableRowNames` _tiles))
  (bind _returnvalue_2 (`|GetDataTableRow` _tiles "Test")
    (:`then`
      (while (< (`local.Index`) (`self.TileCountY`))
        (`KismetSystemLibrary.PrintString` "Hello")
        (`|SpawnActorFromClass` (`.Tile_5_BA01629642787FBBD9EFE5B01477F391` (break `/Game/Levels/ProceduralTileSet/ST_Tile` _returnvalue_2)) (`KismetMathLibrary.MakeTransform` (`KismetMathLibrary.MakeVector` (.x (.location _returnvalue)) (`KismetMathLibrary.Conv_IntToDouble` (* (+ (`local.Index`) 1) (+ (.y (.location _returnvalue)) (`self.TileStandardOffset`)))) (.z (.location _returnvalue))) (.rotation _returnvalue) (.scale _returnvalue)) "Undefined" "MultiplyWithRoot" null null)
        (`/Engine/EditorBlueprintResources/StandardMacros.IncrementInt` (`local.Index`))))))

(fn `UserConstructionScript`)