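; BP_LevelManager is a level streaming manager that starts child level spawning on every BP_LevelSpawn actor.
; The construction script gathers the spawners, and BeginPlay registers each in an ID map before calling SpawnChildLevels.
; ID and parent tracking look unfinished: the index increment is disconnected, parent entries are hardcoded to zero, and ActivateRoom is empty.
; SetActiveRoom only assigns a room when none is valid.
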(event `self.ReceiveBeginPlay`
  (for _array_element (`self.LevelSpawners`)
    (set `self.ActiveRoom` _array_element)
    (`self.SetLevelID` _array_element)
    (`/Game/Levels/LevelStreaming/BP_LevelSpawn.Spawn Child Levels` _array_element)))

(event `SetLevelID`
  (params (Level :type "/Game/Levels/LevelStreaming/BP_LevelSpawn Object Reference"))
  (`BlueprintMapLibrary.Map_Add` (`self.LevelIDs`) Level (`self.IDIndex`))
  (`self.SetParentID` 0))

(event `SetParentID`
  (params (LevelID :type Integer))
  (`BlueprintMapLibrary.Map_Add` (`self.ParentMap`) LevelID))

(event `ActivateRoom`)

(fn `SetActiveRoom`
  (params (NewActiveRoom :type "/Game/Levels/LevelStreaming/BP_LevelSpawn Object Reference"))
  (`self.ActiveRoom`
    (:`then`)
    (:`else`
      (set `self.ActiveRoom` NewActiveRoom))))

(fn `UserConstructionScript`
  ;[1 1 1] Get First Parent
  (bind _outactors (`GameplayStatics.GetAllActorsOfClass` "/Game/Levels/LevelStreaming/BP_LevelSpawn.BP_LevelSpawn_C"))
  (set `self.LevelSpawners` _outactors))