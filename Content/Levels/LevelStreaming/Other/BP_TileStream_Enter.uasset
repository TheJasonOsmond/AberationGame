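; BP_TileStream_Enter is a trigger actor that streams in a sublevel as a level instance when something overlaps its Box.
; A DoOnce gate limits the load to one, placing SubLevel01 at LevelSpawnOffset rotated by the actor's rotation and added to GetLevelTransform's location.
; The instance takes the actor's rotation and its name is printed for debugging, but the SpawnedLevel assignment is disconnected, so no reference is stored.
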(event `self.Box.OnComponentBeginOverlap`
  (params (OverlappedComponent :type "PrimitiveComponent Object Reference") (OtherActor :type "Actor Object Reference") (OtherComp :type "PrimitiveComponent Object Reference") (OtherBodyIndex :type Integer) (bFromSweep :type Boolean) (SweepResult :type "HitResult Structure (by ref)"))
  (bind _returnvalue_location (`KismetMathLibrary.BreakTransform` (`self.GetLevelTransform`)))
  (bind _returnvalue (`self.K2_GetActorRotation`))
  (`/Engine/EditorBlueprintResources/StandardMacros.DoOnce` false
    (:`Completed`
      (`KismetSystemLibrary.PrintString` "Overlap Detected")
      (bind (_boutsuccess _returnvalue_2) (`LevelStreamingDynamic.LoadLevelInstanceBySoftObjectPtr` "/Game/Levels/LevelStreaming/SubLevel01.SubLevel01" (+ _returnvalue_location (* _returnvalue (`self.LevelSpawnOffset`))) _returnvalue "" "/Script/Engine.LevelStreamingDynamic"))
      (`KismetSystemLibrary.PrintString` (`KismetSystemLibrary.GetDisplayName` _returnvalue_2)))))

(fn `UserConstructionScript`)