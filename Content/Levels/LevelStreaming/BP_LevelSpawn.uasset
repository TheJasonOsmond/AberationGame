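; Room trigger actor that streams neighboring level instances as a player moves between rooms.
; Box overlap registers it as the active room with BP_LevelManager, found at construction.
; First entry spawns SubLevel01 instances at each LevelExits transform, maps them by exit and fires LevelCreated.
; Later entries reload those children via ShouldBeLoaded; leaving the box unloads them, despite the Visible/Invisible event names.
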(event `self.Box.OnComponentBeginOverlap`
  (params (OverlappedComponent :type "PrimitiveComponent Object Reference") (OtherActor :type "Actor Object Reference") (OtherComp :type "PrimitiveComponent Object Reference") (OtherBodyIndex :type Integer) (bFromSweep :type Boolean) (SweepResult :type "HitResult Structure (by ref)"))
  ;[1 1 1] Player Entered Level
  (`/Game/Levels/LevelStreaming/BP_LevelManager.SetActiveRoom` (`self.LevelManager`) self)
  (`self.Spawn Child Levels`))

(event `self.Box.OnComponentEndOverlap`
  (params (OverlappedComponent :type "PrimitiveComponent Object Reference") (OtherActor :type "Actor Object Reference") (OtherComp :type "PrimitiveComponent Object Reference") (OtherBodyIndex :type Integer))
  (`self.Set All Children Invisible`))

(event `ReEnterLevel`)

(event `Spawn Child Levels`
  ;[1 1 1] Spawn Child Levels
  (if (`self.NewRoom`)
    (`self.Create Child Levels`)
    (else
      (`self.Set All Children Visible`))))

(event `Create Child Levels`
  ;[1 1 1] Create Child Levels
  (set `self.NewRoom` false)
  (for _array_element (`self.LevelExits`)
    (bind (_boutsuccess _returnvalue) (`LevelStreamingDynamic.LoadLevelInstanceBySoftObjectPtr` "/Game/Levels/LevelStreaming/SubLevel01.SubLevel01" (`self.K2_GetActorLocation` _array_element) (`self.K2_GetActorRotation` _array_element) "" null))
    (`BlueprintMapLibrary.Map_Add` (`self.ChildLevels`) _array_element _returnvalue)
    (`self.LevelCreated`)))

(event `Set All Children Visible`
  (bind _childlevels (`self.ChildLevels`))
  ;[1 1 1] Load Children
  (bind _keys (`BlueprintMapLibrary.Map_Keys` _childlevels))
  (for _array_element _keys
    (set `LevelStreaming.bShouldBeLoaded` true (`BlueprintMapLibrary.Map_Find` _childlevels _array_element))))

(event `Set All Children Invisible`
  (bind _childlevels (`self.ChildLevels`))
  ;[1 1 1] Unload Children
  (bind _keys (`BlueprintMapLibrary.Map_Keys` _childlevels))
  (for _array_element _keys
    (set `LevelStreaming.bShouldBeLoaded` false (`BlueprintMapLibrary.Map_Find` _childlevels _array_element))))

(fn `UserConstructionScript`
  (bind _returnvalue (`GameplayStatics.GetActorOfClass` "/Game/Levels/LevelStreaming/BP_LevelManager.BP_LevelManager_C"))
  (set `self.LevelManager` _returnvalue))